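; BP_EPPQuestDirector is a demo actor that starts the Relic of the Ruins quest when play begins.
; It adds the quest log widget to the first player's viewport and passes that quest's data table row to its QuestLog to accept.
; QuestLog events for objective progress and quest completion print on-screen messages.
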(event OnObjectiveProgress(QuestLog)
  (params (QuestId :type Name :default "None") (ObjectiveId :type Name :default "None"))
  (Development|PrintString "Objective complete!" true true "(R=0.25,G=1.0,B=0.45,A=1.0)" 5.0))

(event OnQuestCompleted(QuestLog)
  (params (QuestId :type Name :default "None"))
  (Development|PrintString "QUEST COMPLETE: Relic of the Ruins" true true "(R=1.0,G=0.82,B=0.22,A=1.0)" 9.0))

(event EventBeginPlay
  (bind _returnvalue (UserInterface|CreateWidget "/EverloreEngine/EverloreEngine/ProjectDemo/Quest/WBP_EPPQuestLog.WBP_EPPQuestLog_C" (Game|GetPlayerController 0)))
  (UserInterface|Viewport|AddtoViewport _returnvalue 0)
  (bind _returnvalue_2 (Utilities|GetDataTableRow (Variables|Default|GetQuestTable) "Q_RelicOfTheRuins")
    (:then
      (Class|EverloreQuestLogComponent|AcceptQuest (Variables|Default|GetQuestLog) (.Quest (Utilities|Struct|BreakEverloreQuestTableRow _returnvalue_2)))
      (Development|PrintString "Quest received: Relic of the Ruins" true true "(R=0.000000,G=0.660000,B=1.000000,A=1.000000)" 8.0))))

(event Collision|EventActorBeginOverlap
  (params (OtherActor :type Actor%20Object%20Reference)))

(event EventTick
  (params (DeltaSeconds :type Float%20%28single-precision%29)))

(fn ConstructionScript)